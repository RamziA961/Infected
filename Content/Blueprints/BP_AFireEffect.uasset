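; Fire effect actor that repeatedly damages any BP_BaseCharacterConfig character overlapping it.
; Begin overlap starts a self-calling, delayed DealFireDamage loop that sends negated DamagePerHit to the character's EventTakeDamage at a rate set by HitsPerSecond.
; A single InContact flag, shared by all overlapping characters, gates the loop and clears when any of them leaves.
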(event Custom|Event%20DealFireDamage
  (params (Other%20Actor :type BP%20Base%20Character%20Config%20Object%20Reference))
  (if (Variables|Default|GetInContact)
    (Default|EventTakeDamage Other%20Actor (* (Variables|Default|GetDamagePerHit) -1))
    (Utilities|FlowControl|Delay (/ 1.0 (Math|Conversions|ToFloat(Integer) (Variables|Default|GetHitsPerSecond))))
    (CallFunction|EventDealFireDamage Other%20Actor)))

(event Collision|EventActorBeginOverlap
  (params (OtherActor :type Actor%20Object%20Reference))
  (bind _asbp_base_character_config (Utilities|Casting|CastToBP_BaseCharacterConfig OtherActor))
  (Variables|Default|SetInContact true)
  (CallFunction|EventDealFireDamage _asbp_base_character_config))

(event Collision|EventActorEndOverlap
  (params (OtherActor :type Actor%20Object%20Reference))
  (Utilities|Casting|CastToBP_BaseCharacterConfig OtherActor)
  (Variables|Default|SetInContact false))

(fn ConstructionScript)