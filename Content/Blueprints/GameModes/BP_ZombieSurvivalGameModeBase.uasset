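; BP_ZombieSurvivalGameModeBase is the zombie survival game mode Blueprint that holds the enemy population cap.
; CanSpawnEnemy reports whether the current enemy count is below MaxEnemies.
; The IncreaseEnemies event waits on a delay, then raises MaxEnemies by a small step while it is under AbsoluteEnemyLimit.
; That event does not loop and nothing in this Blueprint calls it, as BeginPlay and Tick are empty.
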(event Custom|Event%20IncreaseEnemies
  (Utilities|FlowControl|Delay 4e+01)
  (if (< (Variables|Default|GetMaxEnemies) (Variables|Default|GetAbsoluteEnemyLimit))
    (Variables|Default|SetMaxEnemies (+ (Variables|Default|GetMaxEnemies) 2))))

(event EventBeginPlay)

(event EventTick
  (params (DeltaSeconds :type Float%20%28single-precision%29)))

(fn ConstructionScript)

(fn CanSpawnEnemy
  (return (< (Variables|Default|GetNumEnemies) (Variables|Default|GetMaxEnemies))))