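; Zombie enemy that can attack the player and awards a score bounty when killed.
; It initialises its health component on BeginPlay and polls for death on Tick, then ragdolls, adds the bounty to the player's ScoreComponent and destroys itself after a delay.
; AttackPlayer plays an attack montage and, after a timed delay, damages the player's HealthSystem only if the player is in close range and the zombie is still alive.
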(event Custom|Event%20AttackPlayer
  ;[1 1 1] Attack Player Animation and Damage Trigger
  (Animation|Montage|PlayMontage (Variables|Character|GetMesh) "/Game/Animations/Zombie/zombie_attack_Montage.zombie_attack_Montage"
    (:then
      (bind _asbp_base_character_config (Utilities|Casting|CastToBP_BaseCharacterConfig (Game|GetPlayerCharacter 0)))
      (Utilities|FlowControl|Delay 1.55)
      (if (and (<= (Transformation|GetDistanceTo _asbp_base_character_config) 5e+01) (not (Variables|/Game/Blueprints/BP_HealthComponent.BP_HealthComponent_C|GetIsDead (Variables|Default|GetHealthComponent))))
        (Default|AdjustHealth (Variables|/Game/Blueprints/Player/BP_BaseCharacterConfig.BP_BaseCharacterConfig_C|GetHealthSystem _asbp_base_character_config) (* (Variables|Default|GetAttackDamage) -1))))))

(event EventBeginPlay
  (Default|EventUpdateMaxHealth (Variables|Default|GetHealthComponent) (Variables|Default|GetHealth) true))

(event EventTick
  (params (DeltaSeconds :type Float%20%28single-precision%29))
  ;[1 1 1] Death Event
  (if (and (not (Variables|Default|GetDeathTriggered)) (Variables|/Game/Blueprints/BP_HealthComponent.BP_HealthComponent_C|GetIsDead (Variables|Default|GetHealthComponent)))
    (Variables|Default|SetDeathTriggered true)
    (Physics|SetSimulatePhysics (Variables|Character|GetMesh) true)
    ;[1 1 1] Increase Player Score by Zombie's Bounty
    (bind _asbp_base_character_config (Utilities|Casting|CastToBP_BaseCharacterConfig (Game|GetPlayerCharacter 0)))
    (Variables|/Game/Blueprints/BP_ScoreComponent.BP_ScoreComponent_C|SetScore (Variables|/Game/Blueprints/Player/BP_BaseCharacterConfig.BP_BaseCharacterConfig_C|GetScoreComponent _asbp_base_character_config) (+ (Variables|/Game/Blueprints/BP_ScoreComponent.BP_ScoreComponent_C|GetScore (Variables|/Game/Blueprints/Player/BP_BaseCharacterConfig.BP_BaseCharacterConfig_C|GetScoreComponent _asbp_base_character_config)) (Variables|Default|GetScoreBounty)))
    (Utilities|FlowControl|Delay 5.0)
    (Actor|DestroyActor)))

(fn ConstructionScript)