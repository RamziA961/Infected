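; Zombie enemy for a survival game that attacks the player, reacts to hits and awards a score bounty on death.
; HealthComponent holds health; hits play sound and a hurt montage that pauses movement.
; Attacks deal damage after a montage-timed delay if the player is still close.
; Tick detects death once, ragdolls the mesh, updates player score and GameMode's enemy count, stops breathing audio, then destroys the actor after a delay.
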(event Custom|Event%20AttackPlayer
  ;[1 1 1] Attack Player Animation and Damage Trigger
  (Animation|Montage|PlayMontage (Variables|Character|GetMesh) "/Game/Animations/Zombie/zombie_attack_Montage.zombie_attack_Montage"
    (:then
      (bind _asbp_base_character_config (Utilities|Casting|CastToBP_BaseCharacterConfig (Game|GetPlayerCharacter 0)))
      (Utilities|FlowControl|Delay 1.55)
      (if (and (<= (Transformation|GetDistanceTo _asbp_base_character_config) 5e+01) (not (Variables|/Game/Blueprints/BP_HealthComponent.BP_HealthComponent_C|GetIsDead (Variables|Default|GetHealthComponent))))
        (Default|EventTakeDamage _asbp_base_character_config (* (Variables|Default|GetAttackDamage) -1))))))

(event Custom|Event%20PlayDamage
  (bind _charactermovement (Variables|Character|GetCharacterMovement))
  ;[1 1 1] Damage Animation
  (Components|Movement|StopMovementImmediately _charactermovement)
  (Pawn|Components|CharacterMovement|DisableMovement _charactermovement)
  (Animation|Montage|PlayMontage (Variables|Character|GetMesh) "/Game/Animations/Zombie/Hurt_1.Hurt_1"
    (:then
      (Utilities|FlowControl|Delay 1.77)
      (Pawn|Components|CharacterMovement|SetMovementMode (Variables|Character|GetCharacterMovement) "MOVE_Walking" 0))))

(event Custom|Event%20TakeDamage
  (params (Damage :type Integer))
  ;[1 1 1] Damage Audio, Animation, and Health
  (if (not (Variables|Default|GetDeathTriggered))
    (Audio|PlaySoundatLocation "/Game/SoundEffects/Zombie/damage_Cue.damage_Cue" (Transformation|GetActorLocation self) "0, 0, 0" 1.0 1.0 0.0 0 0 0 0)
    (CallFunction|EventPlayDamage)
    (Default|AdjustHealth (Variables|Default|GetHealthComponent) Damage)))

(event Custom|Event%20PlayScreech
  (bind _self self)
  (bind _returnvalue (Transformation|GetActorLocation _self))
  ;[1 1 1] Play Screech on Spawn
  (if (< (Math|Random|RandomFloatinRange 0.0 1.0) 0.2)
    (if (< (Math|Random|RandomFloatinRange 0.0 1.0) 0.5)
      (Audio|PlaySoundatLocation "/Game/SoundEffects/Zombie/screech-1.screech-1" _returnvalue "0, 0, 0" 1.0 1.0 0.0 0 0 0 0)
      (else
        (Audio|PlaySoundatLocation "/Game/SoundEffects/Zombie/screech-2.screech-2" _returnvalue "0, 0, 0" 1.0 1.0 0.0 0 0 0 0)))))

(event Custom|Event%20PlayBreathing
  (bind _breathingaudiocomponent (Variables|Default|GetBreathingAudioComponent))
  ;[1 1 1] Play Heavy Breathing Sound
  (Audio|Components|Audio|SetSound _breathingaudiocomponent "/Game/SoundEffects/Zombie/zombie-breathing_Cue.zombie-breathing_Cue")
  (Audio|Components|Audio|Play _breathingaudiocomponent 0.0))

(event EventBeginPlay
  ;[1 1 1] On Spawn
  (Default|EventUpdateMaxHealth (Variables|Default|GetHealthComponent) (Variables|Default|GetHealth) true)
  (bind _asbp_zombie_survival_game_mode_base (Utilities|Casting|CastToBP_ZombieSurvivalGameModeBase (Game|GetGameMode)))
  (Variables|Default|SetGameMode _asbp_zombie_survival_game_mode_base)
  (CallFunction|EventPlayScreech)
  (CallFunction|EventPlayBreathing))

(event EventTick
  (params (DeltaSeconds :type Float%20%28single-precision%29))
  (bind _gamemode (Variables|Default|GetGameMode))
  ;[1 1 1] Death Event
  (if (and (not (Variables|Default|GetDeathTriggered)) (Variables|/Game/Blueprints/BP_HealthComponent.BP_HealthComponent_C|GetIsDead (Variables|Default|GetHealthComponent)))
    (Variables|Default|SetDeathTriggered true)
    (Physics|SetSimulatePhysics (Variables|Character|GetMesh) true)
    ;[1 1 1] Increase Player Score by Zombie's Bounty
    (bind _asbp_base_character_config (Utilities|Casting|CastToBP_BaseCharacterConfig (Game|GetPlayerCharacter 0)))
    (Variables|/Game/Blueprints/Player/BP_ScoreComponent.BP_ScoreComponent_C|SetScore (Variables|/Game/Blueprints/Player/BP_BaseCharacterConfig.BP_BaseCharacterConfig_C|GetScoreComponent _asbp_base_character_config) (+ (Variables|/Game/Blueprints/Player/BP_ScoreComponent.BP_ScoreComponent_C|GetScore (Variables|/Game/Blueprints/Player/BP_BaseCharacterConfig.BP_BaseCharacterConfig_C|GetScoreComponent _asbp_base_character_config)) (Variables|Default|GetScoreBounty)))
    ;[1 1 1] Decrement Number of Living Enemies
    (Math|Integer|DecrementInt (Variables|/Game/Blueprints/GameModes/BP_ZombieSurvivalGameModeBase.BP_ZombieSurvivalGameModeBase_C|GetNumEnemies _gamemode)
      (:%20%20
        (Variables|/Game/Blueprints/GameModes/BP_ZombieSurvivalGameModeBase.BP_ZombieSurvivalGameModeBase_C|SetNumEnemies _gamemode 0)
        (Audio|Components|Audio|Stop (Variables|Default|GetBreathingAudioComponent))
        (Utilities|FlowControl|Delay 5.0)
        (Actor|DestroyActor)))))

(fn ConstructionScript)