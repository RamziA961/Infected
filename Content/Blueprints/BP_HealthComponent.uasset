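; BP_HealthComponent is an actor component that tracks the owner's integer health between zero and a maximum.
; On BeginPlay it fills health to the maximum and binds to the owner's any-damage event, passing rounded damage into AdjustHealth.
; AdjustHealth applies either a heal or damage, with a nonzero heal taking priority, clamps the result, and calls Death at zero, which only sets an IsDead flag.
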(event Custom|AdjustHealth
  (params (Heal :type Integer) (TakeDamage :type Integer))
  (bind _output_get (Variables|Default|SetHeal Heal))
  (Variables|Default|SetTake%20Damage TakeDamage)
  (if (== _output_get 0)
    (Variables|Default|SetHealthValueModify (* (Variables|Default|GetTake%20Damage) -1))
    (else
      (Variables|Default|SetHealthValueModify (Variables|Default|GetHeal))))
  (Variables|Default|SetCurrentHealth (Math|Integer|Clamp(Integer) (+ (Variables|Default|GetHealthValueModify) (Variables|Default|GetCurrentHealth)) 0 (Variables|Default|GetMaxHealth)))
  (if (<= (Variables|Default|GetCurrentHealth) 0)
    (CallFunction|Death)))

(event Custom|Death
  (Variables|Default|SetIsDead true))

(event Custom|OnTakeAnyDamage
  (params (DamagedActor :type Actor%20Object%20Reference) (Damage :type Float%20%28single-precision%29) (DamageType :type Damage%20Type%20Object%20Reference) (InstigatedBy :type Controller%20Object%20Reference) (DamageCauser :type Actor%20Object%20Reference))
  (CallFunction|AdjustHealth 0 (Math|Float|Round Damage)))

(event EventBeginPlay
  (Variables|Default|SetCurrentHealth (Variables|Default|GetMaxHealth))
  (EventDispatchers|AssignOnTakeAnyDamage (Components|GetOwner) (delegate Custom|OnTakeAnyDamage)))