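; Player inventory component that holds an array of item structs and tracks weapon magazine and reserve rounds.
; AddItem and AddAmmo look up data tables by ID, appending an item or adding rounds to matching entries.
; ConsumeAmmo decrements magazine rounds, but builds from CurrentElement rather than the looped item.
; ReloadAmmo's capped refill logic is disconnected, so its loop changes nothing.
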(event EventBeginPlay
  (bind _asabase_character (Utilities|Casting|CastToABaseCharacter (Components|GetOwner)))
  (Variables|Default|SetPlayer _asabase_character))

(fn AddItem
  (params (ItemID :type Integer))
  (bind _content (Variables|Default|GetContent))
  ;[1 1 1] Add Item To Inventory
  (for _array_element _content
    _)
  (bind _returnvalue (Utilities|GetDataTableRow "/Game/Blueprints/Items/ItemTables/ItemTable.ItemTable" (Utilities|String|StringToName (Utilities|String|ToString(Integer) ItemID)))
    (:then
      (Utilities|Array|Add _content _returnvalue))))

(fn AddAmmo
  (params (AmmoID :type Integer))
  (bind _returnvalue (Utilities|GetDataTableRow "/Game/Blueprints/Items/ItemTables/AmmoTable.AmmoTable" (Utilities|String|StringToName (Utilities|String|ToString(Integer) AmmoID)))
    (:then
      (for (_array_element _array_index) (Variables|Default|GetContent)
        (if (== (.ItemID (Utilities|Struct|BreakFItem _array_element)) (.ItemID (Utilities|Struct|BreakFAmmo _returnvalue)))
          (bind _structout (Utilities|Struct|SetmembersinFItem _array_element (+ (.TotalRounds (Utilities|Struct|BreakFItem _array_element)) (.Rounds (Utilities|Struct|BreakFAmmo _returnvalue)))))
          (Utilities|Array|SetArrayElem (Variables|Default|GetContent) _array_index _structout))))))

(fn ConsumeAmmo
  (params (ItemID :type Integer))
  (for (_array_element _array_index) (Variables|Default|GetContent)
    (LocalVariables|SetCurrentIndex _array_index)
    (if (== (.ItemID (Utilities|Struct|BreakFItem _array_element)) ItemID)
      (bind _structout (Utilities|Struct|SetmembersinFItem (LocalVariables|GetCurrentElement) (- (.MagazineRounds (Utilities|Struct|BreakFItem _array_element)) 1)))
      (Utilities|Array|SetArrayElem (Variables|Default|GetContent) (LocalVariables|GetCurrentIndex) _structout))))

(fn ReloadAmmo
  (params (ItemID :type Integer))
  (for (_array_element _array_index) (Variables|Default|GetContent)
    _))