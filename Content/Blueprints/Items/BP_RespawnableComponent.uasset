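; Actor component that lets its owning item be consumed and then respawn after a delay.
; It caches the owner on BeginPlay.
; Consume hides that actor, disables its collision and starts a one-shot timer for the given hide duration.
; When the timer fires, Respawn unhides the actor and re-enables collision, so the same instance is reused instead of destroyed.
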(event Custom|Event%20Consume
  (params (HideDuration :type Integer))
  ;[1 1 1] Disable Collision For a Duration of Time
  (Utilities|Time|SetTimerbyEvent (delegate Custom|Event%20Respawn) (Math|Conversions|ToFloat(Integer) HideDuration))
  (Rendering|SetActorHiddenInGame (Variables|Default|GetOwner) true)
  (Collision|SetActorEnableCollision (Variables|Default|GetOwner) false))

(event Custom|Event%20Respawn
  ;[1 1 1] Re-Enable Collisions
  (Rendering|SetActorHiddenInGame (Variables|Default|GetOwner) false)
  (Collision|SetActorEnableCollision (Variables|Default|GetOwner) true))

(event EventBeginPlay
  (Variables|Default|SetOwner (Components|GetOwner)))